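; BP_TriDolphin is a dolphin actor, likely ambient sea life, that swims along a spline path.
; Each Tick advances Distance by Speed times delta time plus a fixed per-frame step, then moves the Parent component to that spline point in local space.
; Spline pitch and roll are swapped and negated, and yaw is offset, apparently to align the model with the path.
; When Islooping is set, Distance restarts after passing the spline's end.
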(event `self.ReceiveTick`
  (params (DeltaSeconds :type "Float (single-precision)"))
  (bind _returnvalue (`SplineComponent.GetTransformAtDistanceAlongSpline` (`self.Spline`) (`self.Distance`) "Local" false))
  (set `self.Distance` (+ (* DeltaSeconds (`self.Speed`)) (`self.Distance`) 1.0))
  (`SceneComponent.K2_SetRelativeTransform` (`self.parent`) (`KismetMathLibrary.MakeTransform` (.location _returnvalue) (`KismetMathLibrary.MakeRotator` (* (.pitch (.rotation _returnvalue)) -1.0) (* (.roll (.rotation _returnvalue)) -1.0) (+ (.yaw (.rotation _returnvalue)) 270.0)) (`SceneComponent.RelativeScale3D` (`self.parent`))) false false)
  (if (`self.Islooping`)
    (if (> (`self.Distance`) (`SplineComponent.GetSplineLength` (`self.Spline`)))
      (set `self.Distance` 1.0))))

(fn `UserConstructionScript`)