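; Jellyfish actor that travels along its own spline while its skeletal mesh animates.
; BeginPlay sets the animation play rate from the Fast and Slow flags, with Fast taking priority.
; Tick advances a distance by SplineSpeed and sets the mesh's relative location and rotation from the spline in local space, keeping its scale.
; The distance accumulates without wrapping or resetting.
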(event `self.ReceiveBeginPlay`
  (bind _skeletalmesh (`self.SkeletalMesh`))
  (if (`self.Fast`)
    (`SkeletalMeshComponent.SetPlayRate` _skeletalmesh 1.0)
    (elif (`self.Slow`)
      (`SkeletalMeshComponent.SetPlayRate` _skeletalmesh 0.4))))

(event `self.ReceiveTick`
  (params (DeltaSeconds :type "Float (single-precision)"))
  (bind (_returnvalue_location _returnvalue_rotation) (`KismetMathLibrary.BreakTransform` (`SplineComponent.GetTransformAtDistanceAlongSpline` (`self.Spline`) (`self.Distance Along Spline`) "Local" false)))
  (set `self.Distance Along Spline` (+ (* DeltaSeconds (`self.Spline Speed`)) (`self.Distance Along Spline`)))
  (`SceneComponent.K2_SetRelativeTransform` (`self.SkeletalMesh`) (`KismetMathLibrary.MakeTransform` _returnvalue_location _returnvalue_rotation (`SceneComponent.RelativeScale3D` (`self.SkeletalMesh`))) false false))

(fn `UserConstructionScript`)