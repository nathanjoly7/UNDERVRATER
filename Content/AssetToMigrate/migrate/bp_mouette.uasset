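; Seagull ("mouette") actor Blueprint that moves a skeletal mesh and a box along the actor's spline.
; Each Tick advances a distance by Speed times delta time, plus a fixed per-frame step, and samples the spline in local space.
; The sampled rotation has pitch and roll swapped and negated with a yaw offset, and scale comes from the spline component.
; When Islooping is set, passing the spline's end restarts the path.
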(event `self.ReceiveTick`
  (params (DeltaSeconds :type "Float (single-precision)"))
  (bind _spline (`self.Spline`))
  (bind _returnvalue (`SplineComponent.GetTransformAtDistanceAlongSpline` _spline (`self.Distance`) "Local" false))
  (set `self.Distance` (+ (* (`self.Speed`) DeltaSeconds) (`self.Distance`) 1.0))
  (`SceneComponent.K2_SetRelativeTransform` (`self.SkeletalMesh`) (`KismetMathLibrary.MakeTransform` (.location _returnvalue) (`KismetMathLibrary.MakeRotator` (* (.pitch (.rotation _returnvalue)) -1.0) (* (.roll (.rotation _returnvalue)) -1.0) (+ (.yaw (.rotation _returnvalue)) 270.0)) (`SceneComponent.RelativeScale3D` _spline)) false false)
  (`SceneComponent.K2_SetRelativeTransform` (`self.Box`) (`KismetMathLibrary.MakeTransform` (.location _returnvalue) (`KismetMathLibrary.MakeRotator` (* (.pitch (.rotation _returnvalue)) -1.0) (* (.roll (.rotation _returnvalue)) -1.0) (+ (.yaw (.rotation _returnvalue)) 270.0)) (`SceneComponent.RelativeScale3D` _spline)) false false)
  (if (`self.Islooping`)
    (if (> (`self.Distance`) (`SplineComponent.GetSplineLength` (`self.Spline`)))
      (set `self.Distance` 1.0))))

(fn `UserConstructionScript`)